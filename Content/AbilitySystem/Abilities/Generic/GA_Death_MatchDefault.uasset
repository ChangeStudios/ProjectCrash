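; Default match death ability that switches the dead player to a newly spawned death camera pawn.
; When the triggering event carries a killer pawn, it spawns B_DeathCamPawn at the event target's transform, viewing the killer's root component.
; Otherwise, such as environmental deaths, it copies the level's first B_LevelDeathCamPawn transform into a fresh instance, since each can only be possessed by one player.
; The owning PlayerState's controller then possesses the new camera.
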(event Ability|EventActivateAbilityFromEvent
  (params (EventData :type Gameplay%20Event%20Data%20Structure%20%28by%20ref%29))
  (bind (_eventtag _instigator _target _optionalobject _optionalobject2) (Utilities|Struct|BreakGameplayEventData EventData))
  ;[1 1 1] Spawn and possess a new death camera actor.
  (bind _aspawn (Utilities|Casting|CastToPawn _optionalobject2)
    (:then
      (bind _returnvalue (Game|SpawnActorfromClass "/Game/Player/Pawns/B_DeathCamPawn.B_DeathCamPawn_C" (Transformation|GetActorTransform _target) "Undefined" "MultiplyWithRoot" 0 (Variables|/Script/Engine.Actor|GetRootComponent _aspawn) 0))
      (bind _asplayer_state (Utilities|Casting|CastToPlayerState (Ability|GetOwningActorfromActorInfo)))
      (if (and (Utilities|IsValid _asplayer_state) (Utilities|IsValid (Game|GetPlayerController _asplayer_state)))
        (Pawn|Possess (Game|GetPlayerController _asplayer_state) _returnvalue)))
    (:CastFailed
      ;[1 1 1] If the killer is invalid (e.g. environmental death, fall back to the level's default death camera.
      (bind _outactors (Actor|GetAllActorsOfClass "/Game/Player/Pawns/B_LevelDeathCamPawn.B_LevelDeathCamPawn_C"))
      (Utilities|IsValid (Utilities|Array|Get(acopy) _outactors)
        (:Is%20Valid
          (bind _returnvalue_2 (Game|SpawnActorfromClass "/Game/Player/Pawns/B_LevelDeathCamPawn.B_LevelDeathCamPawn_C" (Transformation|GetActorTransform (Utilities|Array|Get(acopy) _outactors)) "AlwaysSpawn" "MultiplyWithRoot" 0 0)) ; We have to spawn a new camera each time since only one player can possess each one.
          (bind _asplayer_state_2 (Utilities|Casting|CastToPlayerState (Ability|GetOwningActorfromActorInfo)))
          (if (and (Utilities|IsValid _asplayer_state_2) (Utilities|IsValid (Game|GetPlayerController _asplayer_state_2)))
            (Pawn|Possess (Game|GetPlayerController _asplayer_state_2) _returnvalue_2)))))))