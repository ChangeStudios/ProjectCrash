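; Knight Warhammer ability: a ground slam that damages and knocks back nearby characters on landing.
; Activation binds a landed delegate, then applies downward root motion scaled by traced ground distance to keep fall time constant.
; It temporarily equips the hammer, plays dual-perspective montages and fires cues; ending unequips and commits cooldown.
; Landing unbinds, launches overlapped characters, applies SetByCaller damage and fires an impact cue; the line-of-sight check is a placeholder.
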(event Custom|OnLanded
  (params (Hit :type Hit%20Result%20Structure%20%28by%20ref%29))
  (bind _returnvalue (Ability|GetAvatarActorfromActorInfo))
  (bind _knockbackforce (Variables|Ability|GetKnockbackForce))
  (bind _returnvalue_2 (Transformation|GetActorLocation _returnvalue))
  ;[0.2196 0.5 0.5] OnLanded event called when the avatar lands.
  (Utilities|FlowControl|Sequence
    (:then_0
      ;;[0 0.5 0.5] Unbind the OnLanded event to prevent repeated activations.
      (bind _ascharacter (Utilities|Casting|CastToCharacter (Ability|GetAvatarActorfromActorInfo)))
      (EventDispatchers|UnbindEventfromLandedDelegate _ascharacter (EventDispatchers|CreateEvent :!event Custom|OnLanded)))
    (:then_1
      ;;[0 0.5 0.5] Find targets and apply the ability's effects when the avatar lands.
      ;;;[0 0.2205 0.2205] Find characters within the ability's effect radius.
      (bind _outactors (Collision|SphereOverlapActors _returnvalue_2 (Variables|Ability|GetImpactRadius) (Utilities|Array|MakeArray "ObjectTypeQuery3") 0 (Utilities|Array|MakeArray _returnvalue)))
      (for _array_element _outactors
        ;;;[0 0.2205 0.2205] Check if the target has LOS.
        (if true
          ;;;[0 0.2205 0.2205] Launch the target characters away from where the ability-user landed.
          (bind _ascharacter_2 (Utilities|Casting|CastToCharacter _array_element))
          (Character|LaunchCharacter _ascharacter_2 (Math|Vector|MakeVector (.x (* (Math|Vector|GetForwardVector (Class|KismetMathLibrary|NegateRotator (Math|Rotator|FindLookatRotation _returnvalue_2 (Transformation|GetActorLocation _array_element)))) (Math|Vector|MakeVector _knockbackforce (* _knockbackforce -1.0) 0.0))) (.y (* (Math|Vector|GetForwardVector (Class|KismetMathLibrary|NegateRotator (Math|Rotator|FindLookatRotation _returnvalue_2 (Transformation|GetActorLocation _array_element)))) (Math|Vector|MakeVector _knockbackforce (* _knockbackforce -1.0) 0.0))) _knockbackforce) true true)
          ;;;[0 0.2205 0.2205 1 14] Apply the damage effect to the hit target.
          (Utilities|IsValid (Ability|GetAbilitySystemComponent _ascharacter_2)
            (:Is%20Valid
              (bind _returnvalue_3 (Ability|GameplayEffect|AssignTagSetbyCallerMagnitude (Ability|MakeOutgoingGameplayEffectSpec "/Game/AbilitySystem/GameplayEffects/Generic/GE_Damage_Instant_SetByCaller.GE_Damage_Instant_SetByCaller_C") "(TagName=\"Event.SetByCaller.Damage\")" (Variables|Ability|GetDamage)))
              (GameplayEffects|ApplyGameplayEffectSpecToTarget (Ability|GetAbilitySystemComponentfromActorInfo) _returnvalue_3 (Ability|GetAbilitySystemComponent _ascharacter_2)))))))
    (:then_2
      ;;[1 0.3286 0.1582] Trigger the "impact" gameplay cue.
      (Class|GameplayAbility|ExecuteGameplayCuewithParams "(TagName=\"GameplayCue.Knight.Warhammer.Impact.Default\")" (GameplayCue|MakeGameplayCueParametersfromHitResult Hit)))))

(event Ability|EventActivateAbility
  (bind _returnvalue (Ability|GetAbilitySystemComponentfromActorInfo))
  (bind _returnvalue_2 (Ability|GetAvatarActorfromActorInfo))
  (bind _returnvalue_3 (Ability|GetAvatarActorfromActorInfo))
  (bind _returnvalue_4 (Transformation|GetActorLocation _returnvalue_3))
  ;[0.1477 0.1955 1] Check for the ability cooldown.
  (bind _returnvalue_5 (Class|GameplayAbility|CheckAbilityCooldown))
  (if _returnvalue_5
    ;[0 0.5 0] Trigger the ability's effect the next time the character lands.
    (bind _ascharacter (Utilities|Casting|CastToCharacter (Ability|GetAvatarActorfromActorInfo)))
    (EventDispatchers|AssignLandedDelegate _ascharacter (EventDispatchers|CreateEvent :!event Custom|OnLanded))
    ;[0 0.5 0] Get the character's height to determine the force at which they slam down. The force will be scaled to always make the character's fall the same duration.
    (bind _outhit (Collision|LineTraceByChannel _returnvalue_4 (+ _returnvalue_4 "0.000000,0.000000,-1000000.000000") "TraceTypeQuery1" false (Utilities|Array|MakeArray _returnvalue_3) "None"))
    ;[0 0.5 0] Shoot the character to the ground.
    (Ability|Tasks|ApplyRootMotionConstantForce "None" "0.000000,0.000000,-1.000000" (Math|Float|SelectFloat (* (.distance _outhit) (Variables|Default|GetDownwardForceScalar)) 5e+03 (.bblockinghit _outhit)) (Variables|Ability|GetFallDuration) false 0 "ClampVelocity"
      (:then
        (Utilities|FlowControl|Sequence
          (:then_0
            ;[1 0.3286 0.1582] Equip the hammer.
            (bind _asynctaskproxy (|EquipSet "None" (Variables|Default|GetWarhammerEquipmentSet) true))
            (Variables|Default|SetTemporaryEquipTask _asynctaskproxy))
          (:then_1
            ;[1 0.3286 0.1582] Play the first-person and third-person ability animations.
            (|PlayDualMontageandWaitProxy "None" (Variables|Default|GetWarhammerAnimFPP) (Variables|Default|GetWarhammerAnimTPP) 1.0 1.0 "None" "None" false 1.0 0.0 0.0 false
              (:BlendOutDelegate
                _)
              (:InterruptedDelegate
                _)
              (:CancelledDelegate
                _))
            (Class|AbilityTaskEquipSet|UnequipTemporarySet (Variables|Default|GetTemporaryEquipTask)))
          (:then_2
            ;[1 0.3286 0.1582] Trigger the activation gameplay cue.
            (Class|GameplayAbility|ExecuteGameplayCuewithParams "(TagName=\"GameplayCue.Knight.Warhammer.Activate.Default\")" (Ability|GameplayCue|MakeGameplayCueParameters :EffectContext (GameplayEffects|MakeEffectContext _returnvalue) :Location (Transformation|GetActorLocation _returnvalue_2) :Instigator (Components|GetOwner _returnvalue) :EffectCauser _returnvalue_2 :TargetAttachComponent (.firstpersonskeletalmeshcomponent (Class|CrashGameplayAbilityBase|GetCrashActorInfo)))))))
      (:OnFinish
        ;[0 0.5 0] End the ability when the character hits the ground.
        (Ability|EndAbility)))))

(event Ability|EventOnEndAbility
  (params (bWasCancelled :type Boolean))
  ;[1 0 0.09306] Unequip the hammer and start the cooldown when the ability ends.
  (Utilities|FlowControl|Sequence
    (:then_0
      (Class|AbilityTaskEquipSet|UnequipTemporarySet (Variables|Default|GetTemporaryEquipTask)))
    (:then_1
      (Ability|CommitAbilityCooldown false))))