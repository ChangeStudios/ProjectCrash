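; VFX showcase spawner that repeatedly plays a muzzle effect and fires a projectile actor on a timer.
; Tick counts down the muzzle timer, then activates MuzzleFX and, after a projectile delay, spawns the actor, shakes the first player's camera and restarts the countdown.
; The projectile spawns at a mesh-relative gun offset with zero rotation.
; The ready flag clears only after the delay, so muzzle activation repeats each tick until then.
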(event EventTick
  (params (DeltaSeconds :type Float%20%28single-precision%29))
  (Utilities|FlowControl|Sequence
    (:then_0
      ;[1 1 1] Timer
      (if (Variables|Default|Gettimeactivemuzzle)
        (Variables|Default|SetMuzzletimer (- (Variables|Default|GetMuzzletimer) DeltaSeconds))
        (if (<= (Variables|Default|GetMuzzletimer) 0.0)
          (Variables|Default|SetMuzzleready true)
          (Variables|Default|Settimeactivemuzzle false))))
    (:then_1
      ;[1 1 1] Spawn
      (if (Variables|Default|GetMuzzleready)
        (CallFunction|Muzzlefybc)
        (Variables|Default|SetMuzzletimer (Variables|Default|GetMuzzleDelay))
        (Utilities|FlowControl|Delay (Variables|Default|GetProjectileDelay))
        (CallFunction|Spawn)
        (Game|Feedback|ClientStartCameraShake (Game|GetPlayerController 0) "/Game/EditorOnlyAssets/sA_Megapack_v1/sA_Projectilevfx/Vfx/Blueprints/BP_CameraShake01.BP_CameraShake01_C" 3.0 "CameraLocal" "0, 0, 0")
        (Variables|Default|SetMuzzleready false)
        (Variables|Default|Settimeactivemuzzle true)))))

(fn ConstructionScript)

(fn Spawn
  (bind _mesh (Variables|Character|GetMesh))
  (Game|SpawnActorfromClass (Variables|Default|GetActor) (Math|Transform|MakeTransform (+ (Transformation|GetWorldLocation _mesh) (Math|Vector|RotateVector (Variables|Default|GetGunOffset) (Transformation|GetWorldRotation _mesh)))) "AdjustIfPossibleButDontSpawnIfColliding" "SelectDefaultAtRuntime" 0 0) ; Spawn projectile
)

(fn Muzzlefybc
  (bind _muzzle (Variables|Default|GetMuzzle))
  (Class|NiagaraComponent|SetAsset _muzzle (Variables|Default|GetMuzzleFX) true)
  (Components|Activation|SetActive _muzzle true false))