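; BP_ProjectileCluster is a VFX spawner actor that releases a staggered volley of five missile projectiles.
; BeginPlay calls SpawnActor repeatedly, after a short initial wait and then at Delay intervals.
; Each call spawns the Missle class at half scale, randomly scattered around the root in X/Y at a random fixed-range height, offset by Location.
; It passes Rotation and Speed to each missile and applies HueShift through SetColorHue.
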(event EventBeginPlay
  (bind _delay (Variables|Default|GetDelay))
  (Utilities|FlowControl|Delay 0.2)
  (CallFunction|SpawnActor)
  (Utilities|FlowControl|Delay _delay)
  (CallFunction|SpawnActor)
  (Utilities|FlowControl|Delay _delay)
  (CallFunction|SpawnActor)
  (Utilities|FlowControl|Delay _delay)
  (CallFunction|SpawnActor)
  (Utilities|FlowControl|Delay _delay)
  (CallFunction|SpawnActor))

(fn ConstructionScript)

(fn SpawnActor
  (bind _defaultsceneroot (Variables|Default|GetDefaultSceneRoot))
  (bind _returnvalue (Transformation|GetWorldLocation _defaultsceneroot))
  (bind (_x _y) (Math|Vector|BreakVector _returnvalue))
  (bind _returnvalue_2 (Game|SpawnActorfromClass (Variables|Default|GetMissle) (Math|Transform|MakeTransform (+ (Math|Vector|MakeVector (+ _x (Math|Random|RandomFloatinRange -1.5e+02 1.5e+02)) (+ _y (Math|Random|RandomFloatinRange -1.5e+02 1.5e+02)) (+ 7e+02 (Math|Random|RandomFloatinRange 3e+02 8e+02))) (Variables|Default|GetLocation)) (Variables|Default|GetRotation) "0.500000,0.500000,0.500000") "Undefined" "SelectDefaultAtRuntime" 0 (Variables|Default|GetSpeed) 0))
  (Default|SetColorHue _returnvalue_2 (Variables|Default|GetHueShift)))