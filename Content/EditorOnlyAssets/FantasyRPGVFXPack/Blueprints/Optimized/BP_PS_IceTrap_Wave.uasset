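; Ice trap wave VFX actor that pairs a particle system with a timed, animated ice spike crash mesh.
; On BeginPlay it creates dynamic materials for selected emitters, then after short delays spawns a shadow-casting skeletal mesh, plays its crash animation once and later destroys it.
; SetColorHue and SetColorOpacity drive parameters on those materials, with hue also applied to a separate TempCrash component.
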(event EventBeginPlay
  (bind _particlesystem (Variables|Default|GetParticleSystem))
  (for _array_element (Variables|Default|GetEmitterIndexArray)
    (bind _returnvalue (Rendering|Material|CreateDynamicMaterialInstance _particlesystem _array_element (Rendering|Material|GetMaterial _particlesystem _array_element) "None" :!class /Script/Engine.PrimitiveComponent))
    (Utilities|Array|Add (Variables|Default|GetMaterialInstanceArray) _returnvalue))
  (Utilities|FlowControl|Delay 0.8)
  (bind _returnvalue_2 (AddComponent|AddSkeletalMeshComponent false (Math|Transform|MakeTransform (Variables|Default|GetTransform) "0, 0, 0" (Variables|Default|GetScale))))
  (Components|SkinnedMesh|SetSkinnedAssetandUpdate _returnvalue_2 (Variables|Default|GetCrushMesh) true)
  (Rendering|SetCastShadow _returnvalue_2 true)
  (Utilities|FlowControl|Delay 0.3)
  (Components|Animation|PlayAnimation _returnvalue_2 "/Game/EditorOnlyAssets/FantasyRPGVFXPack/Meshes/Spike/Spike_IceCrash_Anim.Spike_IceCrash_Anim" false)
  (Utilities|FlowControl|Delay 3.0)
  (Components|DestroyComponent _returnvalue_2))

(event EventTick
  (params (DeltaSeconds :type Float%20%28single-precision%29)))

(fn ConstructionScript)

(fn SetColorHue
  (params (HueShift :type Float%20%28double-precision%29))
  (bind _tempcrash (Variables|Default|GetTempCrash))
  (for _array_element (Variables|Default|GetMaterialInstanceArray)
    (Rendering|Material|SetScalarParameterValue _array_element "HueShift" HueShift :!class /Script/Engine.MaterialInstanceDynamic))
  (bind _returnvalue (Rendering|Material|CreateDynamicMaterialInstance _tempcrash 0 (Rendering|Material|GetMaterial _tempcrash 0) "None" :!class /Script/Engine.PrimitiveComponent))
  (Rendering|Material|SetScalarParameterValue _returnvalue "HueShift" HueShift :!class /Script/Engine.MaterialInstanceDynamic))

(fn SetColorOpacity
  (params (Opacity :type Float%20%28double-precision%29))
  (for _array_element (Variables|Default|GetMaterialInstanceArray)
    (Rendering|Material|SetScalarParameterValue _array_element "Opacity" Opacity :!class /Script/Engine.MaterialInstanceDynamic)))