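; Ability function library with a helper that picks, from a set of hits, the actor closest to an aim direction.
; Each valid hit actor is scored by the dot product of Aim and its direction from Origin.
; Better-scoring candidates must pass a visibility trace to the impact point and the supplied Gameplay Ability target data filter.
; The best match is returned; the MinimumDot input is never read.
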(fn GetActorClosesttoAim
  (params (Aim :type Vector) (Origin :type Vector) (SourceActor :type Actor%20Object%20Reference) (MinimumDot :type Float%20%28double-precision%29) (Hits :type Array%20of%20Hit%20Result%20Structures) (Filter :type Gameplay%20Target%20Data%20Filter%20Handle%20Structure))
  (for _array_element Hits
    (Utilities|IsValid (.HitActor (Collision|BreakHitResult _array_element))
      (:Is%20Valid
        (LocalVariables|SetItActor (.HitActor (Collision|BreakHitResult _array_element)))
        (if (> (Math|Vector|DotProduct Aim (Math|Vector|Normalize (- (Transformation|GetActorLocation (.HitActor (Collision|BreakHitResult _array_element))) Origin))) (LocalVariables|GetCurrentClosestDot))
          (bind _returnvalue (Collision|LineTraceByChannel SourceActor Origin (.ImpactPoint (Collision|BreakHitResult _array_element)) "TraceTypeQuery1" true (Utilities|Array|MakeArray SourceActor (LocalVariables|GetItActor)) "None"))
          (if (not _returnvalue)
            (if (Ability|TargetData|TargetDataHasActor (Ability|TargetData|FilterTargetData (Ability|TargetData|AbilityTargetDatafromActor (LocalVariables|GetItActor)) Filter))
              (LocalVariables|SetCurrentClosestActor (LocalVariables|GetItActor))
              (LocalVariables|SetCurrentClosestDot (Math|Vector|DotProduct Aim (Math|Vector|Normalize (- (Transformation|GetActorLocation (.HitActor (Collision|BreakHitResult _array_element))) Origin))))))))))
  (return (LocalVariables|GetCurrentClosestActor)))