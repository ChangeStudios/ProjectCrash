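; Knight Parry gameplay ability: a forward dash along the control rotation that damages and knocks back targets caught around the player.
; On activation it checks cooldown, plays first- and third-person montages and applies root motion for the dash.
; A reusable capsule target actor attached to the avatar feeds line-of-sight-checked hits into launch, SetByCaller damage and skin-based impact cues.
; The ability ends when the dash finishes, committing cooldown then.
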(event Ability|EventActivateAbility
  (bind _returnvalue (Ability|GetAvatarActorfromActorInfo))
  (bind _dashduration (Variables|Ability|GetDashDuration))
  ;[0.4381 0.3299 1] Check the ability cooldown.
  (bind _returnvalue_2 (Class|GameplayAbility|CheckAbilityCooldown))
  (if _returnvalue_2
    (Utilities|FlowControl|Sequence
      (:then_0
        ;[0.4381 0.3299 1] Play the first-person and third-person dash animations.
        (|PlayDualMontageandWaitProxy "None" (Variables|Default|GetParryAnimFPP) (Variables|Default|GetParryAnimTPP) 1.0 1.0 "None" "None" false 1.0 0.0 0.0 false))
      (:then_1
        ;[1 0.7597 0.3492] Cache the owning avatar as a character.
        (bind _ascharacter (Utilities|Casting|CastToCharacter (Ability|GetAvatarActorfromActorInfo)))
        (Variables|Default|SetAvatarAsCharacter _ascharacter))
      (:then_2
        ;[0.6824 1 0.916] Spawn the target actor if it does not exist yet.
        (Utilities|IsValid (Variables|Default|GetTargetActor)
          (:Is%20Not%20Valid
            (bind _returnvalue_3 (Game|SpawnActorfromClass :Class "/Script/ProjectCrash.GameplayAbilityTargetActor_CollisionDetector_Capsule" :CollisionHandlingOverride "AlwaysSpawn" :TransformScaleMethod "MultiplyWithRoot" :ReticleClass 0 :Instigator 0))
            (bind _output_get (Variables|Default|SetTargetActor _returnvalue_3))
            (Class|GameplayAbilityTargetActorCollisionDetectorCapsule|Configure _output_get (Variables|Ability|GetCollisionCapsuleRadius) (Variables|Ability|GetCollisionCapsuleHalfHeight) true false true "()" true "(GameplayTags=((TagName=\"State.ImmuneToDamage\")))" true))))
      (:then_3
        ;[0 0.5 0.5 1 14] Search for pawns overlapping this ability's targeting area, which is shaped like a large capsule around the activating player..
        (Transformation|AttachActorToActor (Variables|Default|GetTargetActor) (Ability|GetAvatarActorfromActorInfo) "None" "SnapToTarget" "SnapToTarget" "SnapToTarget" true)
        (bind (_asynctaskproxy _data) (|WaitTargetDatawithReusableActor "CustomMulti" (Variables|Default|GetTargetActor))
          (:then
            (Variables|Default|SetTargetingTask 0 _asynctaskproxy))
          (:ValidDataSentDelegate
            ;[0 0.5 0.5 1 14] Ensure the target has LOS.
            (for _array_element (Ability|TargetData|GetAllActorsfromTargetData _data)
              (Utilities|IsValid _array_element
                (:Is%20Valid
                  (if (Class|AbilitySystemUtilitiesLibrary|ActorHasLineOfSight (Ability|GetAvatarActorfromActorInfo) _array_element "TraceTypeQuery1" true)
                    ;[0 0.5 0.5 1 14] Launch the target in the direction of the activating player's dash.
                    (if (.bSuccess (Utilities|Casting|CastToCharacter _array_element))
                      (Utilities|IsValid (Variables|Default|GetAvatarAsCharacter)
                        (:Is%20Valid
                          (Character|LaunchCharacter (.AsCharacter (Utilities|Casting|CastToCharacter _array_element)) (* (Math|Vector|GetForwardVector (Pawn|GetControlRotation (Variables|Default|GetAvatarAsCharacter) :!class /Script/Engine.Pawn)) (Variables|Ability|GetKnockbackForce)) true true))
                        (:Is%20Not%20Valid
                          _)))
                    ;[0 0.5 0.5 1 14] Apply the damage effect to the hit target.
                    (Utilities|IsValid (Ability|GetAbilitySystemComponent _array_element)
                      (:Is%20Valid
                        (bind _returnvalue_4 (Ability|GameplayEffect|AssignTagSetbyCallerMagnitude (Ability|MakeOutgoingGameplayEffectSpec "/Game/GameplayEffects/Generic/GE_Damage_Instant_SetByCaller.GE_Damage_Instant_SetByCaller_C") "(TagName=\"Event.SetByCaller.Damage\")" (Variables|Ability|GetDamage)))
                        (GameplayEffects|ApplyGameplayEffectSpecToTarget (Ability|GetAbilitySystemComponentfromActorInfo) _returnvalue_4 (Ability|GetAbilitySystemComponent _array_element))
                        ;[0.4381 0.3299 1] Trigger the "impact" gameplay cue.
                        (Class|GameplayAbility|ExecuteGameplayCuewithParams (CallFunction|GetAbilityCuefromSkin "(TagName=\"GameplayCue.Knight.Parry.Impact.Default\")") (Ability|GameplayCue|MakeGameplayCueParameters :EffectContext (GameplayEffects|MakeEffectContext (Ability|GetAbilitySystemComponentfromActorInfo)) :Location (Transformation|GetActorLocation _array_element) :Instigator (Ability|GetAvatarActorfromActorInfo))))))))))))
      (:then_4
        ;[0 0.5 0 1 14] Perform a forward dash on the activating player.
        (Variables|Default|SetOriginalVelocity (Transformation|GetVelocity (Ability|GetAvatarActorfromActorInfo)))
        (Utilities|IsValid (Variables|Default|GetAvatarAsCharacter)
          (:Is%20Valid
            (Ability|Tasks|ApplyRootMotionConstantForce "None" (Math|Vector|GetForwardVector (Pawn|GetControlRotation (Variables|Default|GetAvatarAsCharacter) :!class /Script/Engine.Pawn)) (/ (Variables|Ability|GetDashDistance) _dashduration) _dashduration false 0 "SetVelocity"
              (:OnFinish
                _)))
          (:Is%20Not%20Valid
            _))
        (Ability|EndAbility) ; End the ability after the dash.
      )
      (:then_5
        ;[0.4381 0.3299 1] Trigger the activation gameplay cue.
        (Class|GameplayAbility|ExecuteGameplayCuewithParams (CallFunction|GetAbilityCuefromSkin "(TagName=\"GameplayCue.Knight.Parry.Activate.Default\")") (Ability|GameplayCue|MakeGameplayCueParameters :EffectContext (GameplayEffects|MakeEffectContext (Ability|GetAbilitySystemComponentfromActorInfo)) :Location (Transformation|GetActorLocation _returnvalue) :EffectCauser _returnvalue))))))

(event Ability|EventOnEndAbility
  (params (bWasCancelled :type Boolean))
  ;[0.5 0 0 1 14] Start the cooldown, end the ticking (targeting) task, and clear the list of ignored targets when the ability ends.
  (Ability|CommitAbilityCooldown false)
  (Ability|HasAuthority
    (:True
      (GameplayTasks|EndTask (.TargetingTask (Variables|Default|GetTargetingTask))))
    (:False
      _))
  (Utilities|Array|Clear (Variables|Default|GetTargetsToIgnore)))