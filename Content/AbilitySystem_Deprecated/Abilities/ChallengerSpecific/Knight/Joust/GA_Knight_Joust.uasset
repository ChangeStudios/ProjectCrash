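; Knight Joust ability: temporarily equips a spear and dashes the avatar along the camera's horizontal forward using a root-motion force.
; A reusable, attached capsule target actor detects targets; those in line of sight get knockback, SetByCaller damage and an impact cue.
; Head-on hits with non-pawns end the dash early, locally first to avoid rubber-banding.
; Ending commits the cooldown and unequips the spear; skin-resolved cues provide feedback.
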(event Custom|OnActorHit_Event
  (params (SelfActor :type Actor%20Object%20Reference) (OtherActor :type Actor%20Object%20Reference) (NormalImpulse :type Vector) (Hit :type Hit%20Result%20Structure%20%28by%20ref%29))
  ;[1 0.4535 0.49] End the dash early if the avatar runs into something.
  (if (and (not (Utilities|ClassIsChildOf (Utilities|GetClass OtherActor) "/Script/Engine.Pawn")) (< (Math|Vector|DotProduct (.ImpactNormal (Collision|BreakHitResult Hit)) (Transformation|GetActorForwardVector (Ability|GetAvatarActorfromActorInfo))) -0.15))
    (Ability|EndAbilityLocally) ; Ending the ability without waiting for\nthe server prevents rubber-banding from\nthe "Dash" task.
    (Class|GameplayAbility|ExecuteGameplayCuewithParams (CallFunction|GetAbilityCuefromSkin "(TagName=\"GameplayCue.Knight.Joust.SurfaceImpact.Default\")") (GameplayCue|MakeGameplayCueParametersfromHitResult Hit))
    (Ability|CancelAbility)))

(event Custom|UnbindOnActorHit
  ;[0.06917 1 0.05198] Helper function to unbind OnActorHit.
  (Collision|UnbindEventfromOnActorHit (Ability|GetAvatarActorfromActorInfo) (EventDispatchers|CreateEvent :!event Custom|OnActorHit_Event)))

(event Ability|EventActivateAbility
  (bind _returnvalue (Ability|GetAbilitySystemComponentfromActorInfo))
  (bind _returnvalue_2 (Ability|GetAvatarActorfromActorInfo))
  (bind _dashduration (Variables|Ability|GetDashDuration))
  ;[1 0.9718 0.2727] Check the ability cooldown.
  (bind _returnvalue_3 (Class|GameplayAbility|CheckAbilityCooldown))
  (if _returnvalue_3
    (Utilities|FlowControl|Sequence
      (:then_0
        ;[0.583 1 0.9834] Spawn the target actor if it does not exist yet.
        (Utilities|IsValid (Variables|Default|GetTargetActor)
          (:Is%20Not%20Valid
            (bind _returnvalue_4 (Game|SpawnActorfromClass :Class "/Script/ProjectCrash.GameplayAbilityTargetActor_CollisionDetector_Capsule" :CollisionHandlingOverride "AlwaysSpawn" :TransformScaleMethod "MultiplyWithRoot" :Owner (Ability|GetAvatarActorfromActorInfo) :ReticleClass 0 :Instigator 0))
            (bind _output_get (Variables|Default|SetTargetActor _returnvalue_4))
            (Class|GameplayAbilityTargetActorCollisionDetectorCapsule|Configure _output_get (Variables|Ability|GetCollisionCapsuleRadius) (Variables|Ability|GetCollisionCapsuleHalfHeight) true false true "()" true "(GameplayTags=((TagName=\"State.ImmuneToDamage\")))" true))))
      (:then_1
        ;[0.3773 1 0.7213] Equip the spear.
        (bind _asynctaskproxy (|EquipSet (.SpearEquipmentSet (Variables|Default|GetSpearEquipmentSet)) true))
        (Variables|Default|SetTemporaryEquipTask 0 _asynctaskproxy))
      (:then_2
        ;[1 0.5384 0.2276] Play the first-person and third-person ability animations.
        (|PlayDualMontageandWaitProxy "None" (Variables|Default|GetJoustAnim_FPP) (Variables|Default|GetJoustAnim_TPP) 1.0 1.0 "None" "None" false 1.0 0.0 0.0 false
          (:OnBlendOut
            _)
          (:OnInterrupted
            _)
          (:OnCancelled
            _))
        (CallFunction|UnequipTemporarySet (.TemporaryEquipTask (Variables|Default|GetTemporaryEquipTask))) ; Unequip the spear.
      )
      (:then_3
        ;[0.7851 0.1409 1] Trigger the activation gameplay cue.
        (Class|GameplayAbility|ExecuteGameplayCuewithParams (CallFunction|GetAbilityCuefromSkin "(TagName=\"GameplayCue.Knight.Joust.Activate.Default\")") (Ability|GameplayCue|MakeGameplayCueParameters :EffectContext (GameplayEffects|MakeEffectContext _returnvalue) :Location (Transformation|GetActorLocation _returnvalue_2) :Instigator (Components|GetOwner _returnvalue) :EffectCauser _returnvalue_2)))
      (:then_4
        ;[0.06917 1 0.05198] Dash straight forward in the direction of the camera (disregarding pitch).
        (bind _aschallenger_base (Utilities|Casting|CastTo (Ability|GetAvatarActorfromActorInfo)))
        (bind _asynctaskproxy_2 (Ability|Tasks|ApplyRootMotionConstantForce "None" (Math|Vector|MakeVector (.x (Math|Vector|GetForwardVector (Variables|Default|GetFirstPersonCameraComponent _aschallenger_base))) (.y (Math|Vector|GetForwardVector (Variables|Default|GetFirstPersonCameraComponent _aschallenger_base))) 0.0) (/ (Variables|Ability|GetDashDistance) _dashduration) _dashduration false 0 "SetVelocity")
          (:then
            (Variables|Default|SetDashTask _asynctaskproxy_2)
            ;[0.06917 1 0.05198] Bind the OnActorHit event to detect if the player runs into something during the dash.
            (Collision|AssignOnActorHit (Ability|GetAvatarActorfromActorInfo) (EventDispatchers|CreateEvent :!event Custom|OnActorHit_Event))
            ;[0.06917 1 0.05198] Wait to detect targets with the target actor.
            (Transformation|AttachActorToActor (Variables|Default|GetTargetActor) (Ability|GetAvatarActorfromActorInfo) "None" "SnapToTarget" "SnapToTarget" "SnapToTarget" true)
            (bind (_asynctaskproxy_3 _data) (|WaitTargetDatawithReusableActor "CustomMulti" (Variables|Default|GetTargetActor))
              (:then
                (Variables|Default|SetTargetDetectionTask 0 _asynctaskproxy_3))
              (:ValidDataSentDelegate
                ;[0 0.1615 0.1615] Check for LOS.
                (for _array_element (Ability|TargetData|GetAllActorsfromTargetData _data)
                  (if (Class|AbilitySystemUtilitiesLibrary|ActorHasLineOfSight (Ability|GetAvatarActorfromActorInfo) _array_element "TraceTypeQuery1" true)
                    ;[0 0.1615 0.1615 1 14] Launch the target away from the ability avatar.
                    (bind _ascharacter (Utilities|Casting|CastToCharacter _array_element))
                    (Character|LaunchCharacter _ascharacter (* (Math|Vector|GetForwardVector (Math|Rotator|FindLookatRotation (Transformation|GetActorLocation (Ability|GetAvatarActorfromActorInfo)) (Transformation|GetActorLocation _array_element))) (Variables|Ability|GetKnockbackForce)) true true)
                    ;[0 0.1615 0.1615 1 14] Apply the damage effect to the target.
                    (Utilities|FlowControl|Sequence
                      (:then_0
                        (Utilities|IsValid (Ability|GetAbilitySystemComponent _ascharacter)
                          (:Is%20Valid
                            (bind _returnvalue_5 (Ability|GameplayEffect|AssignTagSetbyCallerMagnitude (Ability|MakeOutgoingGameplayEffectSpec "/Game/GameplayEffects/Generic/GE_Damage_Instant_SetByCaller.GE_Damage_Instant_SetByCaller_C") "(TagName=\"Event.SetByCaller.Damage\")" (Variables|Ability|GetDamage)))
                            (GameplayEffects|ApplyGameplayEffectSpecToTarget (Ability|GetAbilitySystemComponentfromActorInfo) _returnvalue_5 (Ability|GetAbilitySystemComponent _ascharacter)))))
                      (:then_1
                        ;[1 0.1339 0.8657] Trigger the "impact" gameplay cue.
                        (Class|GameplayAbility|ExecuteGameplayCuewithParams (CallFunction|GetAbilityCuefromSkin "(TagName=\"GameplayCue.Knight.Joust.Impact.Default\")") (Ability|GameplayCue|MakeGameplayCueParameters :Location (Transformation|GetActorLocation _array_element))))))))))
          (:OnFinish
            (Ability|EndAbility) ; End the ability after the dash.
          ))))))

(event Ability|EventOnEndAbility
  (params (bWasCancelled :type Boolean))
  (bind _dashtask (Variables|Default|GetDashTask))
  ;[1 0.0685 0.06076] Ability clean-up when it ends.
  (Utilities|FlowControl|Sequence
    (:then_0
      (Ability|CommitAbilityCooldown false) ; Start the ability cooldown.
      (CallFunction|UnbindonActorHit) ; Unbind the OnActorHit event.
    )
    (:then_1
      (CallFunction|UnequipTemporarySet (.TemporaryEquipTask (Variables|Default|GetTemporaryEquipTask))) ; Unequip the spear.
    )
    (:then_2
      ;;[0.3247 0.02224 0.01973] End ongoing tasks.
      (if bWasCancelled
        (GameplayTasks|EndTask (.TargetDetectionTask (Variables|Default|GetTargetDetectionTask)))
        (Utilities|IsValid _dashtask
          (:Is%20Valid
            (GameplayTasks|EndTask _dashtask)))))))